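; Catalyst component that makes its owning flame actor burn, spread fire and burn out.
; A looping Burn timer rolls a spread chance, then runs random line, core sphere and overlap traces, notifying FlammableComponents or spawning ignitors on flammable tags and materials.
; Secondary flames can hop via non-flammable surfaces to find fuel.
; Parent, Child and Tagged ancestry, spacing checks and index caps limit propagation, while lifetime or water extinguishes flames.
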(event `Burn`
  (if (`self.BurnConditions`)
    (`self.IsInWater`
      (:`true`
        (`self.ExtinguishFlame` :!label _label))
      (:`false`
        (`self.CalculateChance` (`self.%ChanceToSpread`)
          (:`Success `
            (`self.Spread`)))))
    (else
      (goto _label))))

(event `self.ReceiveBeginPlay`
  (bind _returnvalue (`self.GetOwner`))
  (bind _life (`self.Life`))
  (bind _burningactor (`self.BurningActor`))
  (`KismetSystemLibrary.Delay` 0.05)
  (`self.CheckAreaToSpawn`
    (:`CannotSpawn`
      (`self.SubtractCurrentFlames` :!label _label_2)
      (`self.BreakFlame`))
    (:`CanSpawn`
      (`self.CheckIndex`
        (:`Break`
          (goto _label_2))
        (:`Valid`
          (`|ExecutionSequence`
            (:`then_0`
              (switch `/Game/CatalystComponent/Blueprints/Enum/Enum_FlameAncestry` (`self.FlameAncestry`)
                (:`NewEnumerator0`
                  (`self.SetParentValues`))
                (:`NewEnumerator1`
                  (`self.ChildSetup`))))
            (:`then_1`
              (`KismetSystemLibrary.K2_SetTimer` null "Burn" (`self.FlameTick`) true)
              (if (not (== _life 0.0))
                (`KismetSystemLibrary.Delay` (+ _life 0.1))
                (`self.ExtinguishLife`)))
            (:`then_2`
              (if (`self.SpawnDecal`)
                (`/Engine/EditorBlueprintResources/StandardMacros.IsValid` _returnvalue
                  (:`Is Valid`
                    (`KismetSystemLibrary.Delay` (`self.TimeBeforeDecalSpawns`))
                    (bind _returnvalue_2 (`|SpawnActorFromClass` "/Game/CatalystComponent/Example/Blueprints/Actors/BurnMark_BP.BurnMark_BP_C" (`KismetMathLibrary.Conv_VectorToTransform` (`Actor.K2_GetActorLocation` _returnvalue)) "Undefined" "OverrideRootScale" _returnvalue null))
                    (`/Game/CatalystComponent/Example/Blueprints/Actors/BurnMark_BP.SetUpDecal` _returnvalue_2 (`self.DecalSize`) (`self.BurnDecalLife`))
                    (`/Engine/EditorBlueprintResources/StandardMacros.IsValid` _burningactor
                      (:`Is Valid`
                        (set `/Game/CatalystComponent/Example/Blueprints/Actors/BurnMark_BP.Actor` _burningactor _returnvalue_2)))))))
            (:`then_3`
              (set `self.FlameSetUpFinished` true))))))))

(event `TagFlameDeath`
  (`KismetSystemLibrary.Delay` (`self.TaggedFlameLife`))
  (`self.TerminateTagged`))

(event `BeginTimer Server`
  (params (actor :type "Actor Object Reference"))
  (`self.BeginTimer Multi` actor))

(event `ToBreak Server`
  (`self.ToBreak Multi`))

(event `BeginTimer Multi`
  (params (Target :type "Actor Object Reference"))
  (`KismetSystemLibrary.Delay` (`self.Life`))
  (`/Engine/EditorBlueprintResources/StandardMacros.IsValid` (`Actor.GetComponentByClass` Target "/Game/CatalystComponent/Blueprints/Components/FlammableComponent_BP.FlammableComponent_BP_C")
    (:`Is Valid`
      (`self.ExtinguishLife`))))

(event `ToBreak Multi`
  (if (`self.CanBeSoftExtinguished`)
    (switch `/Game/CatalystComponent/Blueprints/Enum/Enum_FlameAncestry` (`self.FlameAncestry`)
      (:`NewEnumerator1`
        _)
      (:`NewEnumerator2`
        _))
    (set `self.%ChanceToSpread` 0.0)
    (`KismetSystemLibrary.Delay` 1.5)
    (`self.BreakFlame`)))

(event `GenerateRandomFlameValues Server`
  (bind _returnvalue_x (`KismetMathLibrary.BreakVector` (`Actor.GetActorScale3D` (`self.GetOwner`))))
  (bind _returnvalue (+ (`self.BaseFlameWidth`) 0.0))
  (bind _returnvalue_2 (+ (`self.BaseFlameHeight`) 0.0))
  (bind _returnvalue_3 (/ _returnvalue -1.0))
  (set `self.RandomWidth` (* _returnvalue_x (`KismetMathLibrary.RandomFloatInRange` _returnvalue_3 _returnvalue)))
  (set `self.RandomHeight` (* _returnvalue_x (`KismetMathLibrary.RandomFloatInRange` _returnvalue_3 _returnvalue)))
  (set `self.RandomScale` (* _returnvalue_x (`KismetMathLibrary.RandomFloatInRange` (/ _returnvalue_2 -2.0) _returnvalue_2))))

(fn `BreakFlame`
  (bind _debugtext (`self.DebugText`))
  (`KismetSystemLibrary.PrintString` (`KismetStringLibrary.Concat_StrStr` "Breaking  \"" (`|GetEnumeratorNameAsString` (`self.FlameAncestry`)) "\"  flame") _debugtext _debugtext (struct :`G` 0.66 :`B` 1.0 :`A` 1.0) (`self.DebugDuration`))
  ;[1 0.3325 0.01829 0] Destroy ignition actor
  (switch `/Game/CatalystComponent/Blueprints/Enum/Enum_FlameAncestry` (`self.FlameAncestry`)
    (:`NewEnumerator0`
      (`Actor.K2_DestroyActor` (`self.GetOwner`) :!label _label))
    (:`NewEnumerator1`
      (goto _label))
    (:`NewEnumerator2`
      (`self.TerminateTagged`))))

(fn `CatchFire`
  ;[1 0.3325 0.01829 0] Start up burn loop
  (set `self.ShouldBurn` true)
  (set `self.Extinguish` false)
  (`KismetSystemLibrary.K2_SetTimer` null "Burn" (`self.FlameTick`) true))

(fn `ChildSetup`
  (if (`self.UsedManualChildSetup`)
    _))

(fn `ExtinguishFlame`
  ;[1 0.3325 0.01829 0 13] Ends burn loop. Must use catch fire event to set fire again. If extinguish parent is true catch fire will no longer work because the parent was destroyed
  (if (`self.CanBeSoftExtinguished`)
    (set `self.Extinguish` true)
    (`self.ExtinguishLife`)))

(fn `ExtinguishLife`
  (bind _debugtext (`self.DebugText`))
  (bind (_returnvalue_location _returnvalue_rotation _returnvalue_scale) (`KismetMathLibrary.BreakTransform` (`Actor.GetTransform` (`self.GetOwner`))))
  (`|ExecutionSequence`
    (:`then_0`
      (`/Engine/EditorBlueprintResources/StandardMacros.IsValid` (`self.GetOwner`)
        (:`Is Valid`
          (if (`self.CanBeExtinguished`)
            (`KismetSystemLibrary.PrintString` "Extinguishing" _debugtext _debugtext (struct :`G` 0.66 :`B` 1.0 :`A` 1.0) (`self.DebugDuration`))
            (`GameplayStatics.SpawnEmitterAtLocation` (`self.ExtinguishedSmoke`) _returnvalue_location _returnvalue_rotation _returnvalue_scale)
            (`GameplayStatics.SpawnEmitterAtLocation` (`self.ExtinguishedFlame`) _returnvalue_location _returnvalue_rotation _returnvalue_scale)))))
    (:`then_1`
      (`self.SubtractCurrentFlames`))
    (:`then_2`
      (`self.BreakFlame`))))

(fn `HitTaggedActor`
  (params (Index :type Integer) (SpawnLocation :type "Vector Structure"))
  (if (<= Index (`self.MaxTaggedChildrenPerFlame`))
    (`self.CalculateChance` (`self.%ChanceToSpreadToTags`)
      (:`Success `
        (bind _returnvalue (`|SpawnActorFromClass` (`self.IgnitorSpawnedOnTaggedActor`) (`KismetMathLibrary.Conv_VectorToTransform` SpawnLocation) "Undefined" "OverrideRootScale" null null))
        (`/Engine/EditorBlueprintResources/StandardMacros.IsValid` _returnvalue
          (:`Is Valid`
            (bind _returnvalue_2 (`Actor.GetComponentByClass` _returnvalue "CatalystComponent_BP_C"))
            (`self.SetTagIndex` _returnvalue_2 Index)
            (bind _output_get (set `/Game/CatalystComponent/Blueprints/Components/CatalystComponent_BP.FlameAncestry` "NewEnumerator2" _returnvalue_2))
            (`self.PrepareSpawnedFlame` _returnvalue_2 _output_get _returnvalue)
            (`self.TagFlameDeath` _returnvalue_2)))))))

(fn `LineSpread`
  (bind _secondaryflame_ (`self.SecondaryFlame?`))
  (set `self.SpreadAlready` false)
  (`self.GenerateRandomFlameValues Server`)
  ;[1 0.3325 0.01829 0 14] Preform line trace
  (if (`self.UseLineTraceSpreading`)
    (bind (_hit _value) (`self.LineTraceOwner` (`KismetMathLibrary.MakeVector` (`self.RandomWidth`) (`self.RandomHeight`) (`self.RandomScale`)) (`self.FlammableCollisions`)))
    (if (`self.FalseMaterials` (`.PhysMat` (`GameplayStatics.BreakHitResult` _hit)) _value)
      (`/Engine/EditorBlueprintResources/StandardMacros.IsValid` (`.HitActor` (`GameplayStatics.BreakHitResult` _hit))
        (:`Is Valid`
          (bind (_hit_2 _value_2) (`self.SphereTrace` (`self.MinFlameSpread`) (`.Location` (`GameplayStatics.BreakHitResult` _hit)) (`self.FlameCollision`))) ; Trace for a flame too close
          (`|ExecutionSequence`
            (:`then_0`
              (if (not _value_2)
                (bind _returnvalue (or (`self.ComponentHasTag` (`.HitComponent` (`GameplayStatics.BreakHitResult` _hit)) "flammable") (`Actor.ActorHasTag` (`.HitActor` (`GameplayStatics.BreakHitResult` _hit)) "flammable") (`KismetArrayLibrary.Array_Contains` (`self.FlammableMaterials`) (`.PhysMat` (`GameplayStatics.BreakHitResult` _hit)))))
                (if (not _returnvalue)
                  (bind _returnvalue_2 (`Actor.GetComponentByClass` (`.HitActor` (`GameplayStatics.BreakHitResult` _hit)) "/Game/CatalystComponent/Blueprints/Components/FlammableComponent_BP.FlammableComponent_BP_C"))
                  (`/Engine/EditorBlueprintResources/StandardMacros.IsValid` _returnvalue_2
                    (:`Is Valid`
                      ;;[1 0.3325 0.01829 0 13] Hit target has flammable component
                      (set `self.BurningActor` (`.HitActor` (`GameplayStatics.BreakHitResult` _hit)))
                      (if _secondaryflame_
                        (`/Game/CatalystComponent/Blueprints/Components/FlammableComponent_BP.Hit` _returnvalue_2 (`.Location` (`GameplayStatics.BreakHitResult` _hit)) (`.HitActor` (`GameplayStatics.BreakHitResult` _hit)) (`self.QuickSpread`) (`.HitComponent` (`GameplayStatics.BreakHitResult` _hit)) (+ (`self.ChildIndex`) 1) _secondaryflame_)
                        (`self.ExtinguishLife`)
                        (else
                          (`/Game/CatalystComponent/Blueprints/Components/FlammableComponent_BP.Hit` _returnvalue_2 (`.Location` (`GameplayStatics.BreakHitResult` _hit)) (`.HitActor` (`GameplayStatics.BreakHitResult` _hit)) (`self.QuickSpread`) (`.HitComponent` (`GameplayStatics.BreakHitResult` _hit)) (`self.ChildIndex`) _secondaryflame_)
                          (set `self.SpreadAlready` true :!label _label)))))
                  (else
                    ;;[1 0.3325 0.01829 0 13] Hit target has flammable tag
                    (`/Engine/EditorBlueprintResources/StandardMacros.IsValid` (`.HitComponent` (`GameplayStatics.BreakHitResult` _hit))
                      (:`Is Valid`
                        (if (and _returnvalue (`self.SpreadToTag/PhysicalMaterials`))
                          (if (`self.SecondaryFlame?`)
                            (`self.HitTaggedActor` (+ (`self.TagIndex`) 1) (`.Location` (`GameplayStatics.BreakHitResult` _hit)))
                            (`self.TerminateTagged`)
                            (else
                              (`self.HitTaggedActor` (`self.TagIndex`) (`.Location` (`GameplayStatics.BreakHitResult` _hit)))
                              (goto _label))))))))))
            (:`then_1`
              ;[1 0.3325 0.01829 0 13] This causes the flame to jump to things that are not flammable one time, to see if anything flammable is close by - if you do not want this on a flame - make sure to uncheck "Spread eveywhere" in its component settings and to also set its spawned flames to one that has that unchecked as well.
              (if (and (not (`self.SpreadAlready`)) (`self.SpreadEverywhere`))
                (bind (_hit_3 _value_3) (`self.LineTraceOwner` (`KismetMathLibrary.MakeVector` (`self.RandomWidth`) (`self.RandomHeight`) (`self.RandomScale`)) (`self.FlammableCollisions`)))
                (if _value_3
                  (bind (_hit_4 _value_4) (`self.SphereTrace` (`self.MinFlameSpread`) (`.Location` (`GameplayStatics.BreakHitResult` _hit_3)) (`self.FlameCollision`))) ; Trace for a flame too close
                  (if (not _value_4)
                    (bind _returnvalue_3 (`|SpawnActorFromClass` (`self.SecondarySpreadFlame`) (`KismetMathLibrary.Conv_VectorToTransform` (`.Location` (`GameplayStatics.BreakHitResult` _hit_3))) "AlwaysSpawn" "OverrideRootScale" null null))
                    (bind _returnvalue_4 (`Actor.GetComponentByClass` _returnvalue_3 "CatalystComponent_BP_C"))
                    (`/Engine/EditorBlueprintResources/StandardMacros.IsValid` _returnvalue_4
                      (:`Is Valid`
                        (set `/Game/CatalystComponent/Blueprints/Components/CatalystComponent_BP.ChildIndex` (`self.ChildIndex`) _returnvalue_4)
                        (set `/Game/CatalystComponent/Blueprints/Components/CatalystComponent_BP.SecondaryFlame?` true _returnvalue_4)))))))))))))

(fn `LineSpreadToCollisionType(Example)`
  (set `self.SpreadAlready` false)
  (`self.GenerateRandomFlameValues Server`)
  ;[1 0.3325 0.01829 0 14] Preform line trace
  (if (`self.UseLineTraceSpreading`)
    (bind (_hit _value) (`self.LineTraceOwner` (`KismetMathLibrary.MakeVector` (`self.RandomWidth`) (`self.RandomHeight`) (`self.RandomScale`)) (`|MakeArray` "ObjectTypeQuery7" :!type "EObjectTypeQuery Enum")))
    (if _value
      (bind (_hit_2 _value_2) (`self.SphereTrace` (`self.MinFlameSpread`) (`.Location` (`GameplayStatics.BreakHitResult` _hit)) (`self.FlameCollision`))) ; Trace for a flame too close
      (`|ExecutionSequence`
        (:`then_0`
          (if (not _value_2)
            ;[1 0.3325 0.01829 0 13] Spread to actor since collision is true
            (`self.HitTaggedActor` (+ (`self.TagIndex`) 1) (`.Location` (`GameplayStatics.BreakHitResult` _hit)))))))))

(fn `ManualChildSetup`
  (params (SpreadToActorsWithTag :type Boolean :default true) (QuickSpread :type Boolean) (CastFromCore :type Boolean :default false) (CoreFlameSize :type "Float (double-precision)" :default 30.0) (CanBeExtinguished :type Boolean) (ExtinguishedSmoke :type "ParticleSystem Object Reference") (ExtinguishedFlame :type "ParticleSystem Object Reference") (Life :type "Float (double-precision)" :default 5.0) (MaxChildFlamesOnPlayer :type Integer :default 2) (MaxChildren :type Integer :default 2) (FlameTick :type "Float (double-precision)" :default 0.2) (BaseFlameHeight :type "Float (double-precision)" :default 150.0) (BaseFlameWidth :type "Float (double-precision)" :default 120.0) (MinFlameSpread :type "Float (double-precision)" :default 35.0) (TaggedFlameLife :type "Float (double-precision)" :default 4.0) (IgnitorSpawnedOnTaggedActor :type "Actor Class Reference") (`%ChanceToSpread` :type "Float (double-precision)" :default 60.0))
  (set `self.UsedManualChildSetup` true)
  (set `self.SpreadToTag/PhysicalMaterials` SpreadToActorsWithTag)
  (set `self.QuickSpread` QuickSpread)
  (set `self.UseTraceFromCore` CastFromCore)
  (set `self.CoreFlameSize` CoreFlameSize)
  (set `self.CanBeExtinguished` CanBeExtinguished)
  (set `self.ExtinguishedSmoke` ExtinguishedSmoke)
  (set `self.ExtinguishedFlame` ExtinguishedFlame)
  (set `self.Life` Life)
  (set `self.MaxChildren` MaxChildren)
  (set `self.FlameTick` FlameTick)
  (set `self.BaseFlameHeight` BaseFlameHeight)
  (set `self.BaseFlameWidth` BaseFlameWidth)
  (set `self.MinFlameSpread` MinFlameSpread)
  (set `self.TaggedFlameLife` TaggedFlameLife)
  (set `self.IgnitorSpawnedOnTaggedActor` IgnitorSpawnedOnTaggedActor)
  (set `self.%ChanceToSpread` `%ChanceToSpread`))

(fn `OnOverlapActor`
  (params (`Actor Ref` :type "Actor Object Reference") (Catalyst :type "/Game/CatalystComponent/Blueprints/Components/CatalystComponent_BP Object Reference"))
  (`/Engine/EditorBlueprintResources/StandardMacros.IsValid` (`Actor.GetComponentByClass` `Actor Ref` "/Game/CatalystComponent/Blueprints/Components/FlammableComponent_BP.FlammableComponent_BP_C")
    (:`Is Valid`
      (set `/Game/CatalystComponent/Blueprints/Components/CatalystComponent_BP.BeingOverlapped` true Catalyst))))

(fn `OnOverlapActorEnd`
  (params (Catalyst :type "/Game/CatalystComponent/Blueprints/Components/CatalystComponent_BP Object Reference")))

(fn `OverlapSpread`
  ;[1 0.3325 0.01829 0 13] Spread to overlapping actor if set to
  (if (and (`self.BeingOverlapped`) (`self.UseOverlapSpreading`))
    (`self.SpreadOnTargetLocation` true (`self.OverlappingActor`))))

(fn `PrepareSpawnedFlame`
  (params (Selection :type "/Game/CatalystComponent/Blueprints/Enum/Enum_FlameAncestry Enum" :default "NewEnumerator1") (BurningActor :type "Actor Object Reference"))
  (`/Engine/EditorBlueprintResources/StandardMacros.IsValid` BurningActor
    (:`Is Valid`
      (if (not (`self.CannotSpawn`))
        (switch `/Game/CatalystComponent/Blueprints/Enum/Enum_FlameAncestry` Selection
          (:`NewEnumerator0`
            (set `self.BurningActor` BurningActor))
          (:`NewEnumerator1`
            (set `self.BurningActor` BurningActor))
          (:`NewEnumerator2`
            _))
        (`/Engine/EditorBlueprintResources/StandardMacros.IsValid` BurningActor
          (:`Is Valid`
            (`self.BeginTimer Server` BurningActor)))))))

(fn `SetParentValues`)

(fn `SetTagIndex`
  (params (TagIndex :type Integer))
  (set `self.TagIndex` (+ TagIndex 1)))

(fn `SphereSpread`
  ;[1 0.3325 0.01829 0 12] Preform sphere trace
  (if (`self.UseTraceFromCore`)
    (bind (_hit _value) (`self.SphereTraceOwner` (`self.CoreFlameSize`) (1.0 1.0 1.0) (`self.FlammableCollisions`)))
    (if (`self.FalseMaterials` (`.PhysMat` (`GameplayStatics.BreakHitResult` _hit)) _value)
      (bind _returnvalue (or (`self.ComponentHasTag` (`.HitComponent` (`GameplayStatics.BreakHitResult` _hit)) "flammable") (`Actor.ActorHasTag` (`.HitActor` (`GameplayStatics.BreakHitResult` _hit)) "flammable") (`KismetArrayLibrary.Array_Contains` (`self.FlammableMaterials`) (`.HitActor` (`GameplayStatics.BreakHitResult` _hit)))))
      (if (not _returnvalue)
        (bind _returnvalue_2 (`Actor.GetComponentByClass` (`.HitActor` (`GameplayStatics.BreakHitResult` _hit)) "/Game/CatalystComponent/Blueprints/Components/FlammableComponent_BP.FlammableComponent_BP_C"))
        ;;[1 0.3325 0.01829 0 13] Hit target has flammable component
        (`/Engine/EditorBlueprintResources/StandardMacros.IsValid` _returnvalue_2
          (:`Is Valid`
            (`/Game/CatalystComponent/Blueprints/Components/FlammableComponent_BP.Hit` _returnvalue_2 (`.Location` (`GameplayStatics.BreakHitResult` _hit)) (`.HitActor` (`GameplayStatics.BreakHitResult` _hit)) (`self.QuickSpread`) (`.HitComponent` (`GameplayStatics.BreakHitResult` _hit)) (`self.ChildIndex`) false)))
        (else
          ;;[1 0.3325 0.01829 0 13] Hit target has flammable tag
          (if (and _returnvalue (`self.SpreadToTag/PhysicalMaterials`))
            (`self.HitTaggedActor` (`self.TagIndex`) (`.Location` (`GameplayStatics.BreakHitResult` _hit)))))))))

(fn `Spread`
  (`|ExecutionSequence`
    (:`then_0`
      (`self.LineSpread`))
    (:`then_1`
      (`self.SphereSpread`))
    (:`then_2`
      (`self.OverlapSpread`))))

(fn `SpreadOnTargetLocation`
  (params (SpreadToTaggedActors :type Boolean) (Actor :type "Actor Object Reference"))
  (locals (AlreadySpread :type Boolean))
  (`/Engine/EditorBlueprintResources/StandardMacros.IsValid` Actor
    (:`Is Valid`
      (set `local.AlreadySpread` false)
      (bind (_hit _value) (`self.LineTraceLocation` Actor (2.0 2.0 2.0) (`|MakeArray` "ObjectTypeQuery1" :!type "EObjectTypeQuery Enum")))
      (if _value
        (bind (_hit_2 _value_2) (`self.SphereTrace` (`self.MinFlameSpread`) (`.Location` (`GameplayStatics.BreakHitResult` _hit)) (`self.FlameCollision`))) ; Make sure your ignitor actors are set to the right collision channel. It may be best to give them their own
        (if (not _value_2)
          (`|ExecutionSequence`
            (:`then_0`
              (bind _returnvalue (`Actor.GetComponentByClass` (`.HitActor` (`GameplayStatics.BreakHitResult` _hit)) "/Game/CatalystComponent/Blueprints/Components/FlammableComponent_BP.FlammableComponent_BP_C"))
              ;[1 0.3325 0.01829 0 12] If hit contains component
              (`/Engine/EditorBlueprintResources/StandardMacros.IsValid` _returnvalue
                (:`Is Valid`
                  (`/Game/CatalystComponent/Blueprints/Components/FlammableComponent_BP.Hit` _returnvalue (`.Location` (`GameplayStatics.BreakHitResult` _hit)) (`.HitActor` (`GameplayStatics.BreakHitResult` _hit)) (`self.QuickSpread`) (`.HitComponent` (`GameplayStatics.BreakHitResult` _hit)) (`self.ChildIndex`) false))))
            (:`then_1`
              ;[1 0.3325 0.01829 0 12] If hit contains "flammable" tag
              (if SpreadToTaggedActors
                (if (and (not (`local.AlreadySpread`)) (`Actor.ActorHasTag` (`.HitActor` (`GameplayStatics.BreakHitResult` _hit)) "flammable"))
                  (`self.HitTaggedActor` (`self.TagIndex`) (`.Location` (`GameplayStatics.BreakHitResult` _hit))))))))))))

(fn `SubtractCurrentFlames`
  (bind _burningactor (`self.BurningActor`))
  (bind _returnvalue (`Actor.GetComponentByClass` _burningactor "/Game/CatalystComponent/Blueprints/Components/FlammableComponent_BP.FlammableComponent_BP_C"))
  (`/Engine/EditorBlueprintResources/StandardMacros.IsValid` _burningactor
    (:`Is Valid`
      (`/Engine/EditorBlueprintResources/StandardMacros.IsValid` _returnvalue
        (:`Is Valid`
          (set `/Game/CatalystComponent/Blueprints/Components/FlammableComponent_BP.CurrentFlames` (- (`/Game/CatalystComponent/Blueprints/Components/FlammableComponent_BP.CurrentFlames` _returnvalue) 1) _returnvalue))))))

(fn `TerminateTagged`
  (bind (_returnvalue_location _returnvalue_rotation _returnvalue_scale) (`KismetMathLibrary.BreakTransform` (`Actor.GetTransform` (`self.GetOwner`))))
  (`GameplayStatics.SpawnEmitterAtLocation` (`self.ExtinguishedSmoke`) _returnvalue_location _returnvalue_rotation _returnvalue_scale)
  (`GameplayStatics.SpawnEmitterAtLocation` (`self.ExtinguishedFlame`) _returnvalue_location _returnvalue_rotation _returnvalue_scale)
  (`Actor.K2_DestroyActor` (`self.GetOwner`)))