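; Actor component that makes its owner flammable, tracking fire hits and spreading flames in tandem with CatalystComponent_BP.
; Hit raises burn events past resistance plus durability, then spawns ignitors by collision type, pelvis-attached on pawns, limited by active-flame and extinguish counts.
; Server/Multi event pairs reset counters through cooldown delays, letting actors catch fire again.
; A self-repeating event keeps igniting the owner while in lava.
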(event `self.ReceiveBeginPlay`
  (bind _returnvalue (`self.GetOwner`))
  ;[0.6463 0.3124 1 0] Begin play
  (`/Engine/EditorBlueprintResources/StandardMacros.IsValid` _returnvalue
    (:`Is Valid`
      (set `self.FlammableActor` _returnvalue))))

(event `ResetClearHitTimer Server`
  (`self.ResetClearHit Multi`))

(event `ResetPreventSpread Server`
  (`self.ResetPreventSpreadMulti`))

(event `ResetPreventSpreadMulti`
  (if (not (or (`self.OverlappingFire`) (`self.InLava`)))
    (`KismetSystemLibrary.Delay` (`self.AllowSpreadingCooldown`))
    (set `self.HitCount` 0)
    (set `self.TotalHitCount` 0)))

(event `ResetClearHit Multi`
  (bind _hitcooldown (`self.HitCoolDown`))
  (`KismetSystemLibrary.RetriggerableDelay` _hitcooldown)
  (set `self.HitCount` 0)
  (`self.HitCountReset`)
  (`KismetSystemLibrary.RetriggerableDelay` (- (`self.TotalHitCooldown`) _hitcooldown))
  (set `self.TotalHitCount` 0)
  (`self.TotalHitCountReset`))

(event `PawnInLava Server`
  (`self.PawnInLava Multi`))

(event `PawnInLava Multi`
  (bind _returnvalue (`self.GetOwner`))
  (if (`self.InLava`)
    (bind _returnvalue_2 (`|SpawnActorFromClass` (`self.IgnitorInLava`) (`KismetMathLibrary.Conv_VectorToTransform` (`Actor.K2_GetActorLocation` _returnvalue)) "AlwaysSpawn" "OverrideRootScale" _returnvalue null))
    (bind _returnvalue_3 (`Actor.GetComponentByClass` _returnvalue_2 "/Game/CatalystComponent/Blueprints/Components/CatalystComponent_BP.CatalystComponent_BP_C"))
    (set `/Game/CatalystComponent/Blueprints/Components/CatalystComponent_BP.ChildIndex` 0 _returnvalue_3)
    (`Actor.K2_AttachToActor` _returnvalue_2 _returnvalue "pelvis" "KeepWorld" "KeepRelative" "KeepRelative" true)
    (set `/Game/CatalystComponent/Blueprints/Components/CatalystComponent_BP.FlameAncestry` "NewEnumerator1" _returnvalue_3)
    (`KismetSystemLibrary.Delay` 2.0)
    (`self.PawnInLava Server`)))

(fn `Burned`
  (bind _debug_ (`self.Debug?`))
  ;[0.6463 0.3124 1 0] Every hit to actor this will fire
  (`self.FlameHit`)
  (`self.ResetClearHitTimer Server`)
  ;[0.6463 0.3124 1 0 16] Checks to see if hit count has surpassed durability
  (if (< (+ (`self.Resistance`) (`self.DurabilityToFire`)) (`self.TotalHitCount`))
    (`KismetSystemLibrary.PrintString` "Burn event" _debug_)
    ;[0.6463 0.3124 1 0 13] Calls the event in binded actors
    (`self.BurnEvent`)
    (else
      (`KismetSystemLibrary.PrintString` "Not burned" _debug_))))

(fn `Hit`
  (params (SpawnLocation :type "Vector Structure") (Owner :type "Actor Object Reference") (`QuickSpread?` :type Boolean) (PrimitiveComponent :type "PrimitiveComponent Object Reference") (Index :type Integer) (SecondaryFlame :type Boolean))
  (bind _flammableactor (`self.FlammableActor`))
  (bind _returnvalue (+ (`self.CurrentFlames`) 1))
  (if SecondaryFlame
    (set `self.CurrentFlames` (+ (`self.CurrentFlames`) 1)))
  (if (< _returnvalue (`self.MaxActiveFlames`))
    ;[0.6463 0.3124 1 0] This helps control the fires life
    (if (and (or (<= (`self.HitsUntilExtinguish`) (`self.HitCount`)) (`self.PreventFireSpread`)) (not (`self.InLava`)))
      ;[0.6463 0.3124 1 0] We have to reset that so it can recatch fire later
      (`self.ResetPreventSpread Server`)
      (else
        (`/Engine/EditorBlueprintResources/StandardMacros.IsValid` Owner
          (:`Is Valid`
            (`self.Burned`)
            (set `self.TotalHitCount` (+ (`self.TotalHitCount`) 1))
            (if (not `QuickSpread?`)
              (`self.CheckResistance`))
            (`/Engine/EditorBlueprintResources/StandardMacros.IsValid` Owner
              (:`Is Valid`
                (switch `ECollisionChannel` (`PrimitiveComponent.GetCollisionObjectType` PrimitiveComponent)
                  (:`ECC_WorldStatic`
                    ;[0.6463 0.3124 1 0] Check if it is a pawn being hit or a regular actor
                    (bind _returnvalue_2 (`self.SpawnOnActor` Index (`KismetMathLibrary.Conv_VectorToTransform` SpawnLocation) Owner :!label _label))
                    (`/Engine/EditorBlueprintResources/StandardMacros.IsValid` _returnvalue_2
                      (:`Is Valid`
                        (bind _output_get (set `/Game/CatalystComponent/Blueprints/Components/CatalystComponent_BP.FlameAncestry` "NewEnumerator1" _returnvalue_2))
                        (`/Game/CatalystComponent/Blueprints/Components/CatalystComponent_BP.PrepareSpawnedFlame` _returnvalue_2 _output_get _flammableactor)
                        (if (not (`/Game/CatalystComponent/Blueprints/Components/CatalystComponent_BP.CannotSpawn` _returnvalue_2))
                          (bind _output_get_2 (set `self.CurrentFlames` _returnvalue :!label _label_2))
                          (`KismetSystemLibrary.PrintString` (`KismetStringLibrary.Concat_StrStr` "Active flames: " (`KismetStringLibrary.Conv_IntToString` _output_get_2)) (`self.Debug?`) true (struct :`G` 0.66 :`B` 1.0 :`A` 1.0) 1.0)))))
                  (:`ECC_Pawn`
                    (bind _returnvalue_3 (`self.SpawnOnPawn` Index Owner))
                    (`/Engine/EditorBlueprintResources/StandardMacros.IsValid` _returnvalue_3
                      (:`Is Valid`
                        (bind _output_get_3 (set `/Game/CatalystComponent/Blueprints/Components/CatalystComponent_BP.FlameAncestry` "NewEnumerator1" _returnvalue_3))
                        (`/Game/CatalystComponent/Blueprints/Components/CatalystComponent_BP.PrepareSpawnedFlame` _returnvalue_3 _output_get_3 _flammableactor)
                        (if (not (`/Game/CatalystComponent/Blueprints/Components/CatalystComponent_BP.CannotSpawn` _returnvalue_3))
                          (goto _label_2)))))
                  (:`ECC_Vehicle`
                    (goto _label))
                  (:`ECC_Destructible`
                    (goto _label)))))))))))

(fn `Lava`
  (params (ChildIndex :type Integer) (Owner :type "Actor Object Reference"))
  (bind _returnvalue (`|SpawnActorFromClass` (`self.IgnitorSpawned`) (`KismetMathLibrary.Conv_VectorToTransform` (`Actor.K2_GetActorLocation` Owner)) "AlwaysSpawn" "OverrideRootScale" Owner null))
  (bind _returnvalue_2 (`Actor.GetComponentByClass` _returnvalue "/Game/CatalystComponent/Blueprints/Components/CatalystComponent_BP.CatalystComponent_BP_C"))
  (set `/Game/CatalystComponent/Blueprints/Components/CatalystComponent_BP.ChildIndex` ChildIndex _returnvalue_2)
  (`Actor.K2_AttachToActor` _returnvalue Owner "pelvis" "KeepWorld" "KeepRelative" "KeepRelative" true)
  (set `/Game/CatalystComponent/Blueprints/Components/CatalystComponent_BP.FlameAncestry` "NewEnumerator1" _returnvalue_2))

(fn `SpawnOnActor`
  (params (ChildIndex :type Integer) (SpawnTransform :type "Transform Structure") (Owner :type "Actor Object Reference"))
  (returns (ReturnValue :type "/Game/CatalystComponent/Blueprints/Components/CatalystComponent_BP Object Reference"))
  (bind _ignitorspawned (`self.IgnitorSpawned`))
  (if (`self.SpawnFlameAtRoot`)
    (bind _returnvalue (`|SpawnActorFromClass` _ignitorspawned (`SceneComponent.K2_GetComponentToWorld` (`Actor.RootComponent` Owner)) "AlwaysSpawn" "OverrideRootScale" Owner null))
    (bind _returnvalue_2 (`Actor.GetComponentByClass` _returnvalue "/Game/CatalystComponent/Blueprints/Components/CatalystComponent_BP.CatalystComponent_BP_C"))
    (`/Engine/EditorBlueprintResources/StandardMacros.IsValid` _returnvalue_2
      (:`Is Valid`
        (set `/Game/CatalystComponent/Blueprints/Components/CatalystComponent_BP.ChildIndex` ChildIndex _returnvalue_2)
        (set `/Game/CatalystComponent/Blueprints/Components/CatalystComponent_BP.FlameAncestry` "NewEnumerator1" _returnvalue_2)
        (return _returnvalue_2)))
    (else
      (bind _returnvalue_3 (`|SpawnActorFromClass` _ignitorspawned SpawnTransform "AlwaysSpawn" "OverrideRootScale" Owner null))
      (bind _returnvalue_4 (`Actor.GetComponentByClass` _returnvalue_3 "/Game/CatalystComponent/Blueprints/Components/CatalystComponent_BP.CatalystComponent_BP_C"))
      (`/Engine/EditorBlueprintResources/StandardMacros.IsValid` _returnvalue_4
        (:`Is Valid`
          (set `/Game/CatalystComponent/Blueprints/Components/CatalystComponent_BP.ChildIndex` ChildIndex _returnvalue_4)
          (set `/Game/CatalystComponent/Blueprints/Components/CatalystComponent_BP.FlameAncestry` "NewEnumerator1" _returnvalue_4)
          (return _returnvalue_4))))))

(fn `SpawnOnPawn`
  (params (ChildIndex :type Integer) (Owner :type "Actor Object Reference"))
  (returns (ReturnValue :type "/Game/CatalystComponent/Blueprints/Components/CatalystComponent_BP Object Reference"))
  (bind _returnvalue (`|SpawnActorFromClass` (`self.IgnitorSpawned`) (`KismetMathLibrary.Conv_VectorToTransform` (`Actor.K2_GetActorLocation` Owner)) "AlwaysSpawn" "OverrideRootScale" Owner null))
  (bind _returnvalue_2 (`Actor.GetComponentByClass` _returnvalue "/Game/CatalystComponent/Blueprints/Components/CatalystComponent_BP.CatalystComponent_BP_C"))
  (set `/Game/CatalystComponent/Blueprints/Components/CatalystComponent_BP.ChildIndex` ChildIndex _returnvalue_2)
  (`Actor.K2_AttachToActor` _returnvalue Owner "pelvis" "KeepWorld" "KeepRelative" "KeepRelative" true)
  (set `/Game/CatalystComponent/Blueprints/Components/CatalystComponent_BP.FlameAncestry` "NewEnumerator1" _returnvalue_2)
  (return _returnvalue_2))